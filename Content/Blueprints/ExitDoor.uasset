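; Exit door actor that swings shut, as the entrance behind the player, once any door in the starting room opens.
; At BeginPlay it gathers Door actors whose InputRoom is 0 as the start-room doors.
; Tick polls their IsOpen state, fires CloseDoor on an open one and disables its own tick.
; CloseDoor plays a timeline that lerps the door's relative yaw from Angle to zero.
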(event Custom|CloseDoor
  (bind _newtrack_0 (Timeline|Close PlayFromStart)
    (:Update
      (Transformation|SetRelativeRotation (Variables|Default|GetDoor) (Math|Rotator|MakeRotator 0.0 0.0 (Math|Float|Lerp (Variables|Default|GetAngle) 0.0 _newtrack_0)) false false))))

(event Collision|EventActorBeginOverlap
  (params (OtherActor :type Actor%20Object%20Reference)))

(event EventTick
  (params (DeltaSeconds :type Float%20%28single-precision%29))
  ;[1 1 1] Disable enter door after open any of first doors
  (for _array_element (stale _doors_in_first_room)
    (if (Variables|/Game/Blueprints/Door.Door_C|GetIs%20Open _array_element)
      (CallFunction|CloseDoor)
      (Actor|Tick|SetActorTickEnabled false))))

(fn ConstructionScript)

(event EventBeginPlay
  (bind _doors_in_first_room (Variables|Default|GetDoors%20in%20first%20room))
  (bind _outactors (Actor|GetAllActorsOfClass "/Game/Blueprints/Door.Door_C"))
  (for _array_element _outactors
    (if (== (Variables|/Game/Blueprints/Door.Door_C|GetInput%20Room _array_element) 0)
      (Utilities|Array|Add _doors_in_first_room _array_element)
      (return _doors_in_first_room))))